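; Garage building actor whose gate swings open when the player pawn comes near and closes again when it moves away.
; Tick runs a four-state machine (closed, opening, open, closing) driven by a fixed distance check to the player.
; Open and Close pitch the Gate component a fixed step per frame, so speed depends on frame rate, and advance the state near each angle limit.
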(event EventBeginPlay)

(event EventActorBeginOverlap
  (params (OtherActor :type Actor%20Object%20Reference)))

(event EventTick
  (params (DeltaSeconds :type Float%20%28single-precision%29))
  (bind _returnvalue (Game|Player|GetPlayerPawn 0))
  (bind _returnvalue_2 (Math|Float|MakeLiteralFloat 4e+02))
  (bind _returnvalue_3 (Transformation|GetDistanceTo _returnvalue))
  (switch int (Variables|Default|GetGate_state)
    (:0
      (if (< _returnvalue_3 _returnvalue_2)
        (Variables|Default|SetGate_state 1)
        (CallFunction|Open :!label _label)))
    (:1
      (goto _label))
    (:2
      (if (> _returnvalue_3 _returnvalue_2)
        (Variables|Default|SetGate_state 3)
        (CallFunction|Close :!label _label_2)))
    (:3
      (goto _label_2))))

(fn ConstructionScript)

(fn Open
  (bind _gate (Variables|Default|GetGate))
  (Transformation|AddLocalRotation _gate "-1.000000, 0, 0" false false)
  (if (< (.Pitch (Math|Rotator|BreakRotator (Variables|/Script/Engine.SceneComponent|GetRelativeRotation _gate))) -88.0)
    (Variables|Default|SetGate_state 2)))

(fn Close
  (bind _gate (Variables|Default|GetGate))
  (Transformation|AddLocalRotation _gate "1.000000, 0, 0" false false)
  (if (> (.Pitch (Math|Rotator|BreakRotator (Variables|/Script/Engine.SceneComponent|GetRelativeRotation _gate))) -2.0)
    (Variables|Default|SetGate_state 0)))