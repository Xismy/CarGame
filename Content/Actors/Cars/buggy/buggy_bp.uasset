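; Player-driven buggy vehicle Blueprint with throttle, steering and a nitro boost.
; On BeginPlay it adds a Speedometer widget to the viewport and passes its two flare components to AddFlare.
; Axis inputs feed straight into the vehicle movement component.
; The Nitro press calls a Nitro function, defined outside these graphs, with this car's force, cooldown and duration.
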(event EventBeginPlay
  (bind _returnvalue (UserInterface|CreateWidget "/Game/UI/speedometer.speedometer_C"))
  (UserInterface|Viewport|AddtoViewport _returnvalue 0)
  (Class|Car|AddFlare self (Variables|Default|GetFlare1) (Variables|Default|GetFlare2)))

(event Input|ActionEvents|InputActionNitro
  (params (Key :type Key%20Structure :default "AnyKey"))
  (:Pressed
    (Class|Car|Nitro 5e+06 5.0 0.5)))

(event Input|AxisEvents|InputAxisThrottle
  (params (AxisValue :type Float%20%28single-precision%29))
  (Class|WheeledVehicleMovementComponent|SetThrottleInput (Variables|Default|GetVehicleMovement) AxisValue))

(event Input|AxisEvents|InputAxisSteer
  (params (AxisValue :type Float%20%28single-precision%29))
  (Class|WheeledVehicleMovementComponent|SetSteeringInput (Variables|Default|GetVehicleMovement) AxisValue))

(fn ConstructionScript)